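; Player controller that sets up movement input and handles pause menu and quit hotkeys.
; On BeginPlay it adds the Movement mapping context to the Enhanced Input subsystem.
; Tab uses the Overlay flag to toggle between pausing with a cursor and a new StartMenu widget, and unpausing with the cursor hidden and all widgets removed.
; Escape quits the game immediately.
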(event `self.ReceiveBeginPlay`
  (bind _returnvalue (subsystem `EnhancedInputLocalPlayerSubsystem`))
  (`/Engine/EditorBlueprintResources/StandardMacros.IsValid` _returnvalue
    (:`Is Valid`
      (`EnhancedInputSubsystemInterface.AddMappingContext` _returnvalue "/Game/EnhancedInput/Movement.Movement" 0 (struct)))))

(event `Key|Tab` :paused true
  (params (Key :type "Key Structure"))
  (:`Pressed`
    (if (`self.Overlay`)
      (`GameplayStatics.SetGamePaused` true)
      (set `self.bShowMouseCursor` true)
      (bind _returnvalue (`|CreateWidget` "/Game/HUD/StartMenu.StartMenu_C"))
      (`UserWidget.AddToViewport` _returnvalue 0)
      (set `self.Overlay` false)
      (else
        (`GameplayStatics.SetGamePaused` false)
        (set `self.bShowMouseCursor` false)
        (`WidgetLayoutLibrary.RemoveAllWidgets`)
        (set `self.Overlay` true)))))

(event `Key|Escape`
  (params (Key :type "Key Structure"))
  (:`Pressed`
    (`KismetSystemLibrary.QuitGame` null "Quit")))

(fn `UserConstructionScript`)