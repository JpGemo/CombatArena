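; BP_Player is the player character, handling movement, look, a jetpack, shooting, reloading and ammo clip pickup.
; The jetpack input switches CharacterMovement between Flying, Falling and Walking, adding upward input while flying.
; Shooting spawns a Bullet at the Gun's sphere component, with the Gun found via GetActorOfClass and tracking ammo.
; R reloads an empty Gun, and F collects nearby AmmoClip actors through a distance check.
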(event `EnhancedInput|/Game/EnhancedInput/JetPack`
  (params (ActionValue :type "Float (double-precision)") (ElapsedSeconds :type "Float (double-precision)") (TriggeredSeconds :type "Float (double-precision)") (InputAction :type "InputAction Object Reference" :default "/Game/EnhancedInput/JetPack.JetPack"))
  (:`Triggered`
    (if (`NavMovementComponent.IsFalling` (`self.CharacterMovement`))
      (`CharacterMovementComponent.SetMovementMode` (`self.CharacterMovement`) "MOVE_Flying" 0)
      (else
        (`CharacterMovementComponent.SetMovementMode` (`self.CharacterMovement`) "MOVE_Flying" 0)
        (if (`NavMovementComponent.IsFlying` (`self.CharacterMovement`))
          (`self.AddMovementInput` (`self.GetActorUpVector`) 1.0 true)))))
  (:`Canceled`
    (if (`NavMovementComponent.IsMovingOnGround` (`self.CharacterMovement`))
      (`CharacterMovementComponent.SetMovementMode` (`self.CharacterMovement`) "MOVE_Walking" 0)
      (elif (`NavMovementComponent.IsFalling` (`self.CharacterMovement`))
        (`CharacterMovementComponent.SetMovementMode` (`self.CharacterMovement`) "MOVE_Flying" 0)
        (else
          (`CharacterMovementComponent.SetMovementMode` (`self.CharacterMovement`) "MOVE_Falling" 0)))))
  (:`Completed`
    (`CharacterMovementComponent.SetMovementMode` (`self.CharacterMovement`) "MOVE_Falling" 0)))

(event `EnhancedInput|/Game/EnhancedInput/Look`
  (params (ActionValue :type "Vector2D Structure") (ElapsedSeconds :type "Float (double-precision)") (TriggeredSeconds :type "Float (double-precision)") (InputAction :type "InputAction Object Reference" :default "/Game/EnhancedInput/Look.Look"))
  (:`Triggered`
    (`self.AddControllerYawInput` ActionValue_X)
    (`self.AddControllerPitchInput` ActionValue_Y)))

(event `EnhancedInput|/Game/EnhancedInput/Move`
  (params (ActionValue :type "Vector2D Structure") (ElapsedSeconds :type "Float (double-precision)") (TriggeredSeconds :type "Float (double-precision)") (InputAction :type "InputAction Object Reference" :default "/Game/EnhancedInput/Move.Move"))
  (:`Triggered`
    (`self.AddMovementInput` (`self.GetActorRightVector`) ActionValue_X)
    (`self.AddMovementInput` (`self.GetActorForwardVector`) ActionValue_Y)))

(event `EnhancedInput|/Game/EnhancedInput/Shoot`
  (params (ActionValue :type Boolean) (ElapsedSeconds :type "Float (double-precision)") (TriggeredSeconds :type "Float (double-precision)") (InputAction :type "InputAction Object Reference" :default "/Game/EnhancedInput/Shoot.Shoot"))
  (:`Triggered`
    (bind _returnvalue (`GameplayStatics.GetActorOfClass` "/Game/Objects/Gun.Gun_C"))
    (if (>= (`/Game/Objects/Gun.Ammo` _returnvalue) 1)
      (bind _returnvalue_2 (`GameplayStatics.GetActorOfClass` "/Game/Objects/Gun.Gun_C"))
      (bind _returnvalue_3 (`self.GetComponentByClass` _returnvalue_2 "/Script/Engine.SphereComponent"))
      (`|SpawnActorFromClass` "/Game/Objects/Bullet.Bullet_C" (`KismetMathLibrary.MakeTransform` (`SceneComponent.K2_GetComponentLocation` _returnvalue_3) (`SceneComponent.K2_GetComponentRotation` _returnvalue_3)) "Undefined" "MultiplyWithRoot" null null)
      (bind _returnvalue_4 (`GameplayStatics.GetActorOfClass` "/Game/Objects/Gun.Gun_C"))
      (`/Game/Objects/Gun.ReduceAmmo` _returnvalue_4)
      (else
        (`KismetSystemLibrary.PrintString` "No AMMO")))))

(event `Key|R`
  (params (Key :type "Key Structure"))
  (:`Pressed`
    (bind _returnvalue (`GameplayStatics.GetActorOfClass` "/Game/Objects/Gun.Gun_C"))
    (if (<= (`/Game/Objects/Gun.Ammo` _returnvalue) 0)
      (`/Game/Objects/Gun.ReloadAmmo` _returnvalue))))

(event `Key|F`
  (params (Key :type "Key Structure"))
  (:`Pressed`
    (bind _outactors (`GameplayStatics.GetAllActorsOfClass` "/Game/Objects/AmmoClip.AmmoClip_C"))
    (for (_ _array_index) _outactors
      (bind _output (`|GetArrayItem` _outactors _array_index))
      (if (<= (`KismetMathLibrary.Vector_Distance` (`self.K2_GetActorLocation` _output) (`self.K2_GetActorLocation` (`GameplayStatics.GetPlayerPawn` 0))) 250.0)
        (bind _returnvalue (`GameplayStatics.GetActorOfClass` "/Game/Objects/Gun.Gun_C"))
        (`/Game/Objects/Gun.IncreaseAmmoClip` _returnvalue)
        (`self.K2_DestroyActor` _output)
        (else
          (`KismetSystemLibrary.PrintString` "No Clip Nearby"))))))

(fn `UserConstructionScript`)