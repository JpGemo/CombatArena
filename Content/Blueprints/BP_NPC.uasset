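; BP_NPC is an enemy that chases and shoots at pawns it sees and awards score when destroyed.
; PawnSensing starts an AI move toward the seen pawn, then after a short delay spawns an NPCBullet at the NPCGun transform without waiting for arrival.
; Any actor overlap destroys the NPC.
; On destruction, it adds its Points to the Score in BP_GameMode, found through GetActorOfClass.
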(event OnSeePawn(PawnSensing)
  (params (Pawn :type Pawn%20Object%20Reference))
  (bind _npcgun (Variables|Default|GetNPCGun))
  (AI|AIMoveTo self "0, 0, 0" Pawn 5.0 false
    (:then
      (Utilities|FlowControl|Delay 2.0)
      (Game|SpawnActorfromClass "/Game/Objects/NPCBullet.NPCBullet_C" (Math|Transform|MakeTransform (Transformation|GetWorldLocation _npcgun) (Transformation|GetWorldRotation _npcgun) "1.000000,1.000000,1.000000") "Undefined" "MultiplyWithRoot" 0 0))))

(event Collision|EventActorBeginOverlap
  (params (OtherActor :type Actor%20Object%20Reference))
  (Actor|DestroyActor))

(event EventDestroyed
  (bind _returnvalue (Actor|GetActorOfClass "/Game/Blueprints/BP_GameMode.BP_GameMode_C"))
  (Variables|/Game/Blueprints/BP_GameMode.BP_GameMode_C|SetScore _returnvalue (+ (Variables|/Game/Blueprints/BP_GameMode.BP_GameMode_C|GetScore _returnvalue) (Variables|Default|GetPoints))))

(fn ConstructionScript)