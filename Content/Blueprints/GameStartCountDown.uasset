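; Countdown actor that runs the pre-round countdown and the timed simulation round, showing the seconds on a TextRender.
; Tick uses one-second Delays as its clock, with GameStart and GameActive selecting the phase.
; Round start opens the Door, reloads the Gun and changes fog and lighting.
; The round updates the Score widget and plays voice warnings, then resets environment, gun and player position, sorts high scores and zeroes the score.
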(event `self.ReceiveTick`
  (params (DeltaSeconds :type "Float (single-precision)"))
  (if (`self.GameActive`)
    (`KismetSystemLibrary.Delay` 1.0)
    (`SceneComponent.SetVisibility` (`self.TextRender`) true false)
    (if (> (`self.Timer`) 0)
      (bind _output_get (set `self.Timer` (- (`self.Timer`) 1)))
      (bind _foundwidgets (`WidgetBlueprintLibrary.GetAllWidgetsOfClass` "/Game/HUD/Score.Score_C"))
      (`/Game/HUD/Score.UpdateTimer` _foundwidgets (`KismetTextLibrary.Conv_IntToText` _output_get))
      (`TextRenderComponent.K2_SetText` (`self.TextRender`) (`KismetTextLibrary.Conv_IntToText` (`self.Timer`)))
      (if (== (`self.Timer`) 60)
        (`GameplayStatics.PlaySoundAtLocation` "/Game/Audio/Voice_SixtySecondsRemaining.Voice_SixtySecondsRemaining" (0.0 0.0 0.0) (struct) 1.0 1.0 0.0 null null null null)
        (elif (== (`self.Timer`) 30)
          (`GameplayStatics.PlaySoundAtLocation` "/Game/Audio/Voice_ThirtySecondsRemaining.Voice_ThirtySecondsRemaining" (0.0 0.0 0.0) (struct) 1.0 1.0 0.0 null null null null)
          (elif (== (`self.Timer`) 10)
            (`GameplayStatics.PlaySoundAtLocation` "/Game/Audio/Voice_TenSecondsRemaining.Voice_TenSecondsRemaining" (0.0 0.0 0.0) (struct) 1.0 1.0 0.0 null null null null)
            (elif (== (`self.Timer`) 3)
              (`GameplayStatics.PlaySoundAtLocation` "/Game/Audio/Voice_Three.Voice_Three" (0.0 0.0 0.0) (struct) 1.0 1.0 0.0 null null null null)
              (elif (== (`self.Timer`) 2)
                (`GameplayStatics.PlaySoundAtLocation` "/Game/Audio/Voice_Two.Voice_Two" (0.0 0.0 0.0) (struct) 1.0 1.0 0.0 null null null null)
                (elif (== (`self.Timer`) 1)
                  (`GameplayStatics.PlaySoundAtLocation` "/Game/Audio/Voice_One.Voice_One" (0.0 0.0 0.0) (struct) 1.0 1.0 0.0 null null null null)
                  (elif (== (`self.Timer`) 0)
                    (`GameplayStatics.PlaySoundAtLocation` "/Game/Audio/Voice_SimulationOver.Voice_SimulationOver" (0.0 0.0 0.0) (struct) 1.0 1.0 0.0 null null null null)
                    (bind _returnvalue (`GameplayStatics.GetActorOfClass` "/Script/Engine.ExponentialHeightFog"))
                    (`ExponentialHeightFogComponent.SetFogDensity` (`ExponentialHeightFog.Component` _returnvalue) 0.0)
                    (bind _returnvalue_2 (`GameplayStatics.GetActorOfClass` "/Game/Objects/Gun.Gun_C"))
                    (bind _output_get_2 (set `/Game/Objects/Gun.Ammo` 12 _returnvalue_2))
                    (`TextRenderComponent.K2_SetText` (`/Game/Objects/Gun.AmmoRender` _returnvalue_2) (`KismetTextLibrary.Conv_IntToText` _output_get_2))
                    (set `/Game/Objects/Gun.AmmoClip` 0 _returnvalue_2)
                    (`/Game/Objects/Gun.ReloadAmmo` _returnvalue_2)
                    (set `self.GameActive` false)
                    (bind _returnvalue_3 (`GameplayStatics.GetActorOfClass` "/Script/Engine.DirectionalLight"))
                    (`LightComponent.SetIntensity` (`Light.LightComponent` _returnvalue_3) 1.0)
                    (bind _returnvalue_4 (`GameplayStatics.GetActorOfClass` "/Script/Engine.PlayerStart"))
                    (`self.K2_SetActorLocation` (`GameplayStatics.GetPlayerCharacter` 0) (`self.K2_GetActorLocation` _returnvalue_4) false false)
                    (bind _returnvalue_5 (`GameplayStatics.GetActorOfClass` "/Game/Objects/HighScore.HighScore_C"))
                    (`/Game/Objects/HighScore.SortHighScore` _returnvalue_5)
                    (bind _returnvalue_6 (`GameplayStatics.GetActorOfClass` "/Game/Blueprints/BP_GameMode.BP_GameMode_C"))
                    (set `/Game/Blueprints/BP_GameMode.Score` 0 _returnvalue_6)
                    (set `self.GameActive` false)))))))))
    (else
      (`KismetSystemLibrary.Delay` 1.0)
      (if (`self.GameStart`)
        (`SceneComponent.SetVisibility` (`self.TextRender`) true false)
        (if (> (`self.Timer`) 0)
          (set `self.Timer` (- (`self.Timer`) 1))
          (`TextRenderComponent.K2_SetText` (`self.TextRender`) (`KismetTextLibrary.Conv_IntToText` (`self.Timer`)))
          (if (== (`self.Timer`) 0)
            (set `self.GameStart` false)
            (set `self.GameActive` true)
            (set `self.Timer` 90)
            (`GameplayStatics.PlaySoundAtLocation` "/Game/Audio/Voice_BeginSimulation.Voice_BeginSimulation" (0.0 0.0 0.0) (struct) 1.0 1.0 0.0 null null null null)
            (bind _returnvalue_7 (`GameplayStatics.GetActorOfClass` "/Game/Objects/StartSimulation.StartSimulation_C"))
            (`SceneComponent.SetVisibility` (`/Game/Objects/StartSimulation.Plane` _returnvalue_7) false false)
            (`SceneComponent.SetVisibility` (`self.TextRender`) false false)
            (bind _returnvalue_8 (`GameplayStatics.GetActorOfClass` "/Game/Objects/Gun.Gun_C"))
            (`/Game/Objects/Gun.ReloadAmmo` _returnvalue_8)
            (bind _returnvalue_9 (`GameplayStatics.GetActorOfClass` "/Script/Engine.ExponentialHeightFog"))
            (`ExponentialHeightFogComponent.SetFogDensity` (`ExponentialHeightFog.Component` _returnvalue_9) 5.0)
            (bind _returnvalue_10 (`GameplayStatics.GetActorOfClass` "/Script/Engine.DirectionalLight"))
            (`LightComponent.SetIntensity` (`Light.LightComponent` _returnvalue_10) 1.5)
            (bind _returnvalue_11 (`GameplayStatics.GetActorOfClass` "/Game/Objects/Door.Door_C"))
            (`/Game/Objects/Door.Open` _returnvalue_11)))
        (else
          (`SceneComponent.SetVisibility` (`self.TextRender`) false false)
          (set `self.Timer` 10))))))

(fn `UserConstructionScript`)