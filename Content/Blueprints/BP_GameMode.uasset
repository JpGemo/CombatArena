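; Game mode that sets up the score UI, loads saved high scores and tracks the difficulty modifier.
; On BeginPlay it adds the Score widget, then either copies scores from the "save1" slot into the HighScore actor and sorts them, or creates that save from the actor's scores.
; Tick maps Difficulty to DiffModifier every frame.
; The Scoring event only truncates Score and assigns it back, adding no points.
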(event `self.ReceiveBeginPlay`
  (bind _returnvalue (`|CreateWidget` "/Game/HUD/Score.Score_C"))
  (`UserWidget.AddToViewport` _returnvalue 0)
  (bind _returnvalue_2 (`GameplayStatics.DoesSaveGameExist` "save1"))
  (if _returnvalue_2
    (bind _returnvalue_3 (`GameplayStatics.LoadGameFromSlot` "save1"))
    (bind _asgame_save (cast `/Game/Blueprints/GameSave` _returnvalue_3))
    (bind _returnvalue_4 (`GameplayStatics.GetActorOfClass` "/Game/Objects/HighScore.HighScore_C"))
    (set `/Game/Objects/HighScore.Scores` (`/Game/Blueprints/GameSave.Scores` _asgame_save) _returnvalue_4)
    (`/Game/Objects/HighScore.SortHighScore` _returnvalue_4)
    (else
      (bind _returnvalue_5 (`GameplayStatics.CreateSaveGameObject` "/Game/Blueprints/GameSave.GameSave_C"))
      (bind _returnvalue_6 (`GameplayStatics.GetActorOfClass` "/Game/Objects/HighScore.HighScore_C"))
      (set `/Game/Blueprints/GameSave.Scores` (`/Game/Objects/HighScore.Scores` _returnvalue_6) _returnvalue_5)
      (`GameplayStatics.SaveGameToSlot` _returnvalue_5 "save1"))))

(event `self.ReceiveTick`
  (params (DeltaSeconds :type "Float (single-precision)"))
  (if (== (`self.Difficulty`) 1)
    (set `self.DiffModifier` 1.0)
    (elif (== (`self.Difficulty`) 2)
      (set `self.DiffModifier` 0.75)
      (elif (== (`self.Difficulty`) 3)
        (set `self.DiffModifier` 0.5)))))

(event `Scoring`
  (set `self.Score` (`KismetMathLibrary.FTrunc` (`KismetMathLibrary.Conv_IntToDouble` (`self.Score`)))))

(fn `UserConstructionScript`)